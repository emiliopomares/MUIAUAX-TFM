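; Cell actor that records whether anything overlaps it and shows that occupancy through its cube's material.
; BeginPlay gives the Cube a dynamic material instance.
; Each Capture call refreshes overlaps on demand, checks the collision component for overlapping actors, then sets the Occupancy flag and switches the Density parameter between on and off values.
; An "already occupied" debug branch is left unconnected.
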(event Custom|Capture
  (Class|OverlapDetector|UpdateOverlaps)
  (if (> (Utilities|Array|Length (Collision|GetOverlappingActors (Variables|Default|GetMyCollisionComponent) 0 :!class /Script/Engine.PrimitiveComponent)) 0)
    (Rendering|Material|SetScalarParameterValue (stale EventBeginPlay _returnvalue) "Density" (Variables|Default|GetOnDensity) :!class /Script/Engine.MaterialInstanceDynamic)
    (Variables|Default|SetOccupancy true)
    (else
      (Rendering|Material|SetScalarParameterValue (stale EventBeginPlay _returnvalue) "Density" (Variables|Default|GetOffDensity) :!class /Script/Engine.MaterialInstanceDynamic)
      (Variables|Default|SetOccupancy false))))

(event EventBeginPlay
  (bind _returnvalue (Rendering|Material|CreateDynamicMaterialInstance (Variables|Default|GetCube) 0 0 "None" :!class /Script/Engine.PrimitiveComponent))
  (Rendering|Material|SetMaterial (Variables|Default|GetCube) 0 _returnvalue))

(event Collision|EventActorBeginOverlap
  (params (OtherActor :type Actor%20Object%20Reference)))

(event EventTick
  (params (DeltaSeconds :type Float%20%28single-precision%29)))

(fn ConstructionScript)
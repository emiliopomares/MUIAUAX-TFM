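; SingleBook3 is a book scene object with three alternative components, one named ProbabilisticRobotics.
; Its disconnected graph logic would randomly show one at the origin and teleport the other two far below, then call Prepare and the parent Setup.
; The Setup event is empty, so that selection never runs and the parent Setup is not called from it.
; The construction script only calls its parent.
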(event EventSetup)

(fn ConstructionScript
  (|CallParentFunction))
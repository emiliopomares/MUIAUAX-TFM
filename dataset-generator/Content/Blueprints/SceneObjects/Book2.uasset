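; Book2 is a scene object Blueprint that shows one of three book variants at random: OrbitalMechanics, DataDriven or ProbabilisticRobotics.
; Its Setup event rolls a random index, teleports the chosen component to the local origin and hides the other two by dropping them far below.
; It then calls Prepare and the parent Setup, while the construction script only runs the parent's.
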(event EventSetup
  (bind _orbitalmechanics (Variables|Default|GetOrbitalMechanics))
  (bind _datadriven (Variables|Default|GetDataDriven))
  (bind _probabilisticrobotics (Variables|Default|GetProbabilisticRobotics))
  (switch int (Math|Random|RandomIntegerinRange 0 2)
    (:Default
      _)
    (:0
      (Transformation|SetRelativeLocation _orbitalmechanics "0.000000,0.000000,-10000.000000" false true)
      (Transformation|SetRelativeLocation _datadriven "0.000000,0.000000,-10000.000000" false true)
      (Transformation|SetRelativeLocation _probabilisticrobotics "0, 0, 0" false true))
    (:1
      (Transformation|SetRelativeLocation _orbitalmechanics "0, 0, 0" false true)
      (Transformation|SetRelativeLocation _datadriven "0.000000,0.000000,-10000.000000" false true)
      (Transformation|SetRelativeLocation _probabilisticrobotics "0.000000,0.000000,-10000.000000" false true))
    (:2
      (Transformation|SetRelativeLocation _orbitalmechanics "0.000000,0.000000,-10000.000000" false true)
      (Transformation|SetRelativeLocation _datadriven "0, 0, 0" false true)
      (Transformation|SetRelativeLocation _probabilisticrobotics "0.000000,0.000000,-10000.000000" false true)))
  (CallFunction|Prepare)
  (|CallParentFunction))

(fn ConstructionScript
  (|CallParentFunction))
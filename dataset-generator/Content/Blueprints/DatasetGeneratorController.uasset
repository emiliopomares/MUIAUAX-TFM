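; Controller that generates a dataset of stereo camera images paired with camera pose and occupancy field data.
; An endless delayed loop repositions actors through ObjectPlacer, times the CellManager capture, then calls Prepare on all EventListener actors.
; Each data point packs pose floats and the camera-relative occupancy field into a numbered binary file alongside exported images.
; An empty output path shows a warning widget and disables writing.
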(event Custom|GatherDataPoint
  (bind _stereocamera (Variables|References|GetStereoCamera))
  (bind _outpath (Variables|Default|GetOutPath))
  ;[1 1 1] Gather Data Point
  (for _array_element (Variables|Default|GetEventListeners)
    (Default|Prepare _array_element))
  (bind _pose (Default|GetPose _stereocamera))
  (bind _field (Default|GetOccupancyField (Variables|References|GetCellManager) _stereocamera))
  (Utilities|FlowControl|Sequence
    (:then_0
      (bind _outdata (Class|BPFileIO|ConvertFloattoByteArray (.X (Utilities|Struct|BreakPose _pose)))))
    (:then_1
      (bind _outdata_2 (Class|BPFileIO|ConvertFloattoByteArray (.Y (Utilities|Struct|BreakPose _pose)))))
    (:then_2
      (bind _outdata_3 (Class|BPFileIO|ConvertFloattoByteArray (.Z (Utilities|Struct|BreakPose _pose)))))
    (:then_3
      (bind _outdata_4 (Class|BPFileIO|ConvertFloattoByteArray (.qx (Utilities|Struct|BreakPose _pose)))))
    (:then_4
      (bind _outdata_5 (Class|BPFileIO|ConvertFloattoByteArray (.qy (Utilities|Struct|BreakPose _pose)))))
    (:then_5
      (bind _outdata_6 (Class|BPFileIO|ConvertFloattoByteArray (.qz (Utilities|Struct|BreakPose _pose)))))
    (:then_6
      (bind _outdata_7 (Class|BPFileIO|ConvertFloattoByteArray (.qw (Utilities|Struct|BreakPose _pose)))))
    (:then_7
      (Utilities|FlowControl|Sequence
        (:then_0
          (Utilities|Array|AppendArray _outdata _outdata_2))
        (:then_1
          (Utilities|Array|AppendArray _outdata _outdata_3))
        (:then_2
          (Utilities|Array|AppendArray _outdata _outdata_4))
        (:then_3
          (Utilities|Array|AppendArray _outdata _outdata_5))
        (:then_4
          (Utilities|Array|AppendArray _outdata _outdata_6))
        (:then_5
          (Utilities|Array|AppendArray _outdata _outdata_7))
        (:then_6
          (Utilities|Array|AppendArray _outdata _field)
          (if (Utilities|Enum|NotEqual(Enum) _outpath "")
            (Default|ExportImageData _stereocamera _outpath (Variables|Default|GetFrameCount))
            (Class|BPFileIO|WriteBytestoFile (Utilities|String|Append _outpath "/" (Utilities|String|ToString(Integer) (Variables|Default|GetFrameCount)) "T.bin") _outdata)
            (Variables|Default|SetFrameCount (+ (Variables|Default|GetFrameCount) 1))
            (else
              (Development|PrintString "OUTPUT DISABLED"))))))))

(event EventBeginPlay
  (if (Utilities|Enum|Equal(Enum) (Variables|Default|GetOutPath) "")
    (bind _returnvalue (UserInterface|CreateWidget "/Game/UI/NoOutputWarning.NoOutputWarning_C"))
    (UserInterface|Viewport|AddtoViewport _returnvalue 0))
  (bind _outactors (Actor|GetAllActorsOfClass "/Game/Blueprints/EventListener.EventListener_C"))
  (Variables|Default|SetEventListeners _outactors)
  (Development|PrintString (Utilities|String|ToString(Integer) (Utilities|Array|Length _outactors)))
  (Utilities|FlowControl|Delay 0.5)
  (Default|PositionActors (Variables|References|GetObjectPlacer) :!label _label)
  (Utilities|FlowControl|Delay (Variables|Default|GetCooldown))
  (Class|KismetAnimationLibrary|StartProfilingTimer)
  (Default|Capture (Variables|References|GetCellManager))
  (bind _returnvalue_2 (Class|KismetAnimationLibrary|EndProfilingTimer true))
  (Development|PrintString (Utilities|String|Append "Took " (Utilities|String|ToString(Float) (/ _returnvalue_2 1e+03)) " seconds"))
  (CallFunction|GatherDataPoint)
  (Utilities|FlowControl|Delay 0.2)
  (goto _label))

(fn ConstructionScript)
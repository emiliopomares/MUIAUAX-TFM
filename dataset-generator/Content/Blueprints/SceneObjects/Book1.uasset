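; Book scene object that randomizes its appearance and layout each time its Setup event runs.
; Setup scatters and yaws the Cube, sinking it out of sight half the time, and gives StaticMesh3 a random material through RandomMaterialMesh.
; It randomly shows one of three named book components, hiding the others by teleporting them far below rather than toggling visibility.
; It then calls Prepare and the parent Setup.
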(event EventBeginPlay
  (|CallParentFunction) ; This node is disabled and will not be called.\nDrag off pins to build functionality.
)

(event Collision|EventActorBeginOverlap
  (params (OtherActor :type Actor%20Object%20Reference))
  (|CallParentFunction OtherActor) ; This node is disabled and will not be called.\nDrag off pins to build functionality.
)

(event EventTick
  (params (DeltaSeconds :type Float%20%28single-precision%29))
  (|CallParentFunction DeltaSeconds) ; This node is disabled and will not be called.\nDrag off pins to build functionality.
)

(event EventSetup
  (bind _returnvalue (Math|Random|RandomUnitVector))
  (bind _orbitalmechanics (Variables|Default|GetOrbitalMechanics))
  (bind _datadriven (Variables|Default|GetDataDriven))
  (bind _probabilisticrobotics (Variables|Default|GetProbabilisticRobotics))
  (bind _returnvalue_2 (* _returnvalue "60.000000,60.000000,0.000000"))
  (bind (_x _y) (Math|Vector|BreakVector _returnvalue_2))
  ;[1 1 1] SetUpCube
  (Transformation|SetRelativeLocationAndRotation (Variables|Default|GetCube) (Math|Vector|MakeVector _x _y (Math|Float|SelectFloat 2.2 -1e+04 (< (Math|Random|RandomFloatinRange 0.0 1.0) 0.5))) (Math|Rotator|MakeRotator 0.0 0.0 (Math|Random|RandomFloatinRange 0.0 359.0)) false true)
  (Default|ChooseRandomMaterial (Variables|Default|GetRandomMaterialMesh) (Variables|Default|GetStaticMesh3))
  (switch int (Math|Random|RandomIntegerinRange 0 2)
    (:Default
      (Transformation|SetRelativeLocation _orbitalmechanics "0.000000,0.000000,-10000.000000" false true :!label _label)
      (Transformation|SetRelativeLocation _datadriven "0.000000,0.000000,0.000000" false true)
      (Transformation|SetRelativeLocation _probabilisticrobotics "0.000000,0.000000,-10000.000000" false true))
    (:0
      (Transformation|SetRelativeLocation _orbitalmechanics "0.000000,0.000000,-10000.000000" false true)
      (Transformation|SetRelativeLocation _datadriven "0.000000,0.000000,-10000.000000" false true)
      (Transformation|SetRelativeLocation _probabilisticrobotics "0.000000,0.000000,0.000000" false true))
    (:1
      (Transformation|SetRelativeLocation _orbitalmechanics "0.000000,0.000000,0.000000" false true)
      (Transformation|SetRelativeLocation _datadriven "0.000000,0.000000,-10000.000000" false true)
      (Transformation|SetRelativeLocation _probabilisticrobotics "0.000000,0.000000,-10000.000000" false true))
    (:2
      (goto _label)))
  (CallFunction|Prepare)
  (|CallParentFunction))

(fn ConstructionScript
  (|CallParentFunction))
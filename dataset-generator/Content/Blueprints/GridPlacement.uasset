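; GridPlacement is an actor Blueprint that moves itself to a random position and rotation within set limits.
; CaptureMin and CaptureMax store the actor's current location as the two corners of the allowed volume.
; Prepare picks a random point in that box and teleports the actor there.
; Rotation reuses the random-point-in-box technique on MinRotation and MaxRotation, mapping X, Y and Z to roll, pitch and yaw.
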(event Custom|Capture%20Min
  (Variables|Default|SetMinPos (Transformation|GetActorLocation)))

(event Custom|Capture%20Max
  (Variables|Default|SetMaxPos (Transformation|GetActorLocation)))

(event EventBeginPlay)

(event Collision|EventActorBeginOverlap
  (params (OtherActor :type Actor%20Object%20Reference)))

(event EventTick
  (params (DeltaSeconds :type Float%20%28single-precision%29)))

(event EventPrepare
  (bind _maxrotation (Variables|Default|GetMaxRotation))
  (bind _minrotation (Variables|Default|GetMinRotation))
  (bind _minrotation_2 (Variables|Default|GetMinRotation))
  (bind _maxrotation_2 (Variables|Default|GetMaxRotation))
  (bind _returnvalue (- _maxrotation _minrotation))
  (bind _returnvalue_2 (+ _maxrotation_2 _minrotation_2))
  (bind _returnvalue_3 (* _returnvalue_2 "0.500000,0.500000,0.500000"))
  (bind _returnvalue_4 (* _returnvalue "0.500000,0.500000,0.500000"))
  (bind _returnvalue_5 (Math|Random|RandomPointinBoundingBox _returnvalue_3 _returnvalue_4))
  (bind (_x _y _z) (Math|Vector|BreakVector _returnvalue_5))
  (Transformation|SetActorLocationAndRotation (Math|Random|RandomPointinBoundingBox (* (+ (Variables|Default|GetMaxPos) (Variables|Default|GetMinPos)) "0.500000,0.500000,0.500000") (* (- (Variables|Default|GetMaxPos) (Variables|Default|GetMinPos)) "0.500000,0.500000,0.500000")) (Math|Rotator|MakeRotator _x _y _z)))

(fn ConstructionScript)
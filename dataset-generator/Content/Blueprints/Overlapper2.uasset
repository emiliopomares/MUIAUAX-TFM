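; Overlapper2 is a debug actor that periodically reports which actors overlap its collision component.
; After BeginPlay it waits two seconds, then runs a repeating delay loop that fires the custom Capture event at the same interval.
; Capture calls UpdateOverlaps, then prints each overlapping actor's display name to screen, or a colored "Nothing here" message when none are found.
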(event Custom|Capture
  (bind _mycollisioncomponent (Variables|Default|GetMyCollisionComponent))
  (bind _overlappingactors (Collision|GetOverlappingActors _mycollisioncomponent 0 :!class /Script/Engine.PrimitiveComponent))
  (Class|OverlapDetector|UpdateOverlaps)
  (if (== (Utilities|Array|Length _overlappingactors) 0)
    (Development|PrintString "Nothing here" true true "(R=0.989147,G=0.188569,B=1.000000,A=1.000000)")
    (else
      (for _array_element _overlappingactors
        (Development|PrintString (Utilities|GetDisplayName _array_element))))))

(event EventBeginPlay
  (Utilities|FlowControl|Delay 2.0)
  (CallFunction|Capture :!label _label)
  (Utilities|FlowControl|Delay 2.0)
  (goto _label))

(event Collision|EventActorBeginOverlap
  (params (OtherActor :type Actor%20Object%20Reference)))

(event EventTick
  (params (DeltaSeconds :type Float%20%28single-precision%29)))

(fn ConstructionScript)
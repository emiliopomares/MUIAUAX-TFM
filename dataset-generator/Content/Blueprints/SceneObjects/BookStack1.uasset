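; BookStack1 is a scene object Blueprint for a stack of three books that gets a slightly different, untidy arrangement on Setup.
; Each book component receives a small random horizontal offset and yaw, keeping its height while resetting pitch and roll.
; Setup then calls Prepare and the parent Setup, while the construction script only runs the parent's.
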(event EventSetup
  (bind _returnvalue (Math|Random|RandomUnitVector))
  (bind _returnvalue_2 (Math|Random|RandomFloatinRange -2e+01 2e+01))
  (bind _orbitalmechanics (Variables|Default|GetOrbitalMechanics))
  (bind _datadriven (Variables|Default|GetDataDriven))
  (bind _probabilisticrobotics (Variables|Default|GetProbabilisticRobotics))
  (bind _returnvalue_3 (Math|Rotator|MakeRotator 0.0 0.0 _returnvalue_2))
  (bind _returnvalue_4 (* _returnvalue "5.000000,5.000000,0.000000"))
  (Transformation|SetRelativeLocation _orbitalmechanics (+ _returnvalue_4 (Math|Vector|MakeVector 0.0 0.0 (.Z (Math|Vector|BreakVector (Variables|/Script/Engine.SceneComponent|GetRelativeLocation _orbitalmechanics))))) false false)
  (Transformation|SetRelativeLocation _datadriven (+ _returnvalue_4 (Math|Vector|MakeVector 0.0 0.0 (.Z (Math|Vector|BreakVector (Variables|/Script/Engine.SceneComponent|GetRelativeLocation _datadriven))))) false false)
  (Transformation|SetRelativeLocation _probabilisticrobotics (+ _returnvalue_4 (Math|Vector|MakeVector 0.0 0.0 (.Z (Math|Vector|BreakVector (Variables|/Script/Engine.SceneComponent|GetRelativeLocation _probabilisticrobotics))))) false false)
  (Transformation|SetRelativeRotation (Variables|Default|GetProbabilisticRobotics) _returnvalue_3 false false)
  (Transformation|SetRelativeRotation (Variables|Default|GetOrbitalMechanics) _returnvalue_3 false false)
  (Transformation|SetRelativeRotation (Variables|Default|GetDataDriven) _returnvalue_3 false false)
  (CallFunction|Prepare)
  (|CallParentFunction))

(fn ConstructionScript
  (|CallParentFunction))
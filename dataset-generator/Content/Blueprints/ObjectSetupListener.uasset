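; ObjectSetupListener is an actor that responds to Setup, Hide and Prepare events for a placed object.
; Setup calls ParentPrepare, applies a random yaw, and prints a separately rolled random value, so the log does not match the applied rotation.
; Hide teleports the actor below the world origin rather than changing visibility.
; BeginPlay caches the starting Z, unused here, and Prepare only prints a do-nothing message.
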(event Custom|Setup
  (bind _returnvalue (Math|Random|RandomFloatinRange 0.0 359.0))
  ;[1 1 1] Setup object and rotate around Z axis
  (|CallParentFunction)
  (Transformation|SetActorRotation (Math|Rotator|MakeRotator 0.0 0.0 _returnvalue))
  (Development|PrintString (Utilities|String|Append "Rotate: " (Utilities|String|ToString(Float) _returnvalue))))

(event Custom|Hide
  ;[1 1 1] Hide
  (Transformation|SetActorLocation "0.000000,0.000000,-1000.000000" false true))

(event EventBeginPlay
  (Variables|Default|SetOriginZ (.Z (Math|Vector|BreakVector (Transformation|GetActorLocation)))))

(event EventPrepare
  (Development|PrintString "DOING NOTHING"))

(fn ConstructionScript)
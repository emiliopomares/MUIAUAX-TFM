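; SolidCell is a cell actor that detects whether something overlaps its cube and exposes the result as an occupancy value.
; Shortly after BeginPlay, it checks the cube's overlapping actors once, then sets Occupancy to full or empty.
; A dynamic material instance's Density parameter mirrors that state, showing the cell as dense or faint.
; GetOccupancy returns the stored value; an unconnected branch that would hide the cube never runs.
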(event EventBeginPlay
  (bind _returnvalue (Rendering|Material|CreateDynamicMaterialInstance (Variables|Default|GetCube) 0 "/Game/3DModels/Materials/CellMaterial.CellMaterial" "None" :!class /Script/Engine.PrimitiveComponent))
  (Rendering|Material|SetMaterial (Variables|Default|GetCube) 0 _returnvalue)
  (Utilities|FlowControl|Delay 0.2)
  (if (> (Utilities|Array|Length (Collision|GetOverlappingActors (Variables|Default|GetCube) 0 :!class /Script/Engine.PrimitiveComponent)) 0)
    (Rendering|Material|SetScalarParameterValue _returnvalue "Density" 0.95 :!class /Script/Engine.MaterialInstanceDynamic)
    (Variables|Default|SetOccupancy 127)
    (else
      (Rendering|Material|SetScalarParameterValue _returnvalue "Density" 0.04 :!class /Script/Engine.MaterialInstanceDynamic)
      (Variables|Default|SetOccupancy 0))))

(fn ConstructionScript)

(fn GetOccupancy
  (return (Variables|Default|GetOccupancy)))
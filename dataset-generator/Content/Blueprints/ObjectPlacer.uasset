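; Object placer Blueprint that randomizes which items appear on a table.
; PositionActors hides every entry in Objects, then calls Setup on randomly picked entries, with repeats possible, using a count drawn from NumberOfItemsOnTable.
; The debug print draws its own random count, so it can differ from the loop's.
; Unconnected leftover graphs hold a timed repeat loop and random transform logic; nothing here calls PositionActors at runtime.
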(event Custom|PositionActors
  (bind _numberofitemsontable (Variables|Default|GetNumberOfItemsOnTable))
  (bind _returnvalue (Utilities|Array|Length _numberofitemsontable))
  (bind _returnvalue_2 (- _returnvalue 1))
  (bind _returnvalue_3 (Math|Random|RandomIntegerinRange 0 _returnvalue_2))
  (bind _output (Utilities|Array|Get(acopy) _numberofitemsontable _returnvalue_3))
  ;[1 1 1] Place variable number of items on table
  (for _array_element (Variables|References|GetObjects)
    (Default|Hide _array_element))
  (Development|PrintString (Utilities|String|ToString(Integer) _output) true true "(R=0.869170,G=0.000000,B=1.000000,A=1.000000)")
  (for _index (range 0 _output)
    (Default|Setup (Utilities|Array|Get(acopy) (Variables|References|GetObjects) (Math|Random|RandomIntegerinRange 0 (- (Utilities|Array|Length (Variables|References|GetObjects)) 1))))))

(event EventBeginPlay)

(event Collision|EventActorBeginOverlap
  (params (OtherActor :type Actor%20Object%20Reference)))

(event EventTick
  (params (DeltaSeconds :type Float%20%28single-precision%29)))

(fn ConstructionScript)
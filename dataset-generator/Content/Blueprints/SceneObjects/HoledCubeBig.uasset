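; HoledCubeBig is a scene object Blueprint that randomizes its look and layout when its Setup event runs.
; Setup gives each of its two static meshes a random material from the Materials array.
; A coin flip keeps either SceneUpRight or SceneFront at zero relative location and teleports the other far below, switching variants by offset rather than visibility.
; It then calls the parent Setup, while construction only calls the parent.
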(event EventBeginPlay
  (|CallParentFunction) ; This node is disabled and will not be called.\nDrag off pins to build functionality.
)

(event Collision|EventActorBeginOverlap
  (params (OtherActor :type Actor%20Object%20Reference))
  (|CallParentFunction OtherActor) ; This node is disabled and will not be called.\nDrag off pins to build functionality.
)

(event EventTick
  (params (DeltaSeconds :type Float%20%28single-precision%29))
  (|CallParentFunction DeltaSeconds) ; This node is disabled and will not be called.\nDrag off pins to build functionality.
)

(event EventSetup
  (bind _materials (Variables|Default|GetMaterials))
  (bind _returnvalue (Utilities|Array|Length _materials))
  (bind _returnvalue_2 (- _returnvalue 1))
  (bind _returnvalue_3 (Math|Random|RandomIntegerinRange 0 _returnvalue_2))
  (bind _output (Utilities|Array|Get(acopy) _materials _returnvalue_3))
  (Rendering|Material|SetMaterial (Variables|Default|GetStaticMesh) 0 _output)
  (Rendering|Material|SetMaterial (Variables|Default|GetStaticMesh1) 0 _output)
  (Variables|Default|Setpicka (< (Math|Random|RandomFloatinRange 0.0 1.0) 0.5))
  (Transformation|SetRelativeLocation (Variables|Default|GetSceneUpRight) (Math|Vector|MakeVector 0.0 0.0 (Math|Float|SelectFloat -1e+04 0.0 (Variables|Default|Getpicka))) false true)
  (Transformation|SetRelativeLocation (Variables|Default|GetSceneFront) (Math|Vector|MakeVector 0.0 0.0 (Math|Float|SelectFloat 0.0 -1e+04 (Variables|Default|Getpicka))) false true)
  (|CallParentFunction))

(fn ConstructionScript
  (|CallParentFunction))